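; BP_MoveCube is an actor that bobs up and down along the Z axis in a smooth sine wave.
; Each Tick adds the scaled change in sine of time since creation over the frame to its current height, so no start position is stored.
; The move sets location without sweep, and BeginPlay, overlap and the construction script are empty.
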(event EventBeginPlay)

(event Collision|EventActorBeginOverlap
  (params (OtherActor :type Actor%20Object%20Reference)))

(event EventTick
  (params (DeltaSeconds :type Float%20%28single-precision%29))
  (bind _returnvalue (Actor|GetGameTimeSinceCreation))
  (bind _returnvalue_2 (Transformation|GetActorLocation))
  (bind (_x _y _z) (Math|Vector|BreakVector _returnvalue_2))
  (Variables|Default|SetDeltaSeconds DeltaSeconds)
  (Transformation|SetActorLocation (Math|Vector|MakeVector _x _y (+ _z (* (- (Math|Trig|Sin(Radians) (+ _returnvalue (Variables|Default|GetDeltaSeconds))) (Math|Trig|Sin(Radians) _returnvalue)) 5e+01))) false false))

(fn ConstructionScript)